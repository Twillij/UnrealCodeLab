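; Player Blueprint that runs branching conversations as a dialogue participant, supplying its name, icon and gender.
; On BeginPlay it creates a collapsed UI_Dialogue widget, which StartDialogue and SelectDialogueOption refresh from the active dialogue context.
; Entering dialogue disables player input and shows the cursor with Game and UI input, and ending it reverses this.
; Condition, value and event handlers are stubs, and Tick prints the dialogue state for debugging.
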(event `self.ReceiveBeginPlay`
  (bind _returnvalue (`|CreateWidget` "/Game/Widgets/UI_Dialogue.UI_Dialogue_C" (`GameplayStatics.GetPlayerController` 0)))
  (bind _output_get (set `self.DialogueWidget` _returnvalue))
  (`UserWidget.AddToViewport` _output_get 0)
  (`Widget.SetVisibility` _output_get "Collapsed"))

(event `self.ReceiveTick`
  (params (DeltaSeconds :type "Float (single-precision)"))
  (if (`self.bInDialogue`)
    (`KismetSystemLibrary.PrintString` "In Dialogue" true true (struct :`G` 0.66 :`B` 1.0 :`A` 1.0) 0.0)
    (else
      (`KismetSystemLibrary.PrintString` "Not In Dialogue" true true (struct :`G` 0.66 :`B` 1.0 :`A` 1.0) 0.0))))

(fn `CheckCondition`
  (params (Context :type "DlgContext Object Reference") (ConditionName :type Name))
  (returns (ReturnValue :type Boolean))
  (return false))

(fn `GetBoolValue`
  (params (ValueName :type Name))
  (returns (ReturnValue :type Boolean))
  (return false))

(fn `GetFloatValue`
  (params (ValueName :type Name))
  (returns (ReturnValue :type "Float (double-precision)"))
  (return 0.0))

(fn `GetIntValue`
  (params (ValueName :type Name))
  (returns (ReturnValue :type Integer))
  (return 0))

(fn `GetNameValue`
  (params (ValueName :type Name))
  (returns (ReturnValue :type Name))
  (return "None"))

(fn `GetParticipantDisplayName`
  (params (ActiveSpeaker :type Name))
  (returns (ReturnValue :type Text))
  (return (`KismetTextLibrary.Conv_NameToText` (`self.PlayerName`))))

(fn `GetParticipantGender`
  (returns (ReturnValue :type "ETextGender Enum"))
  (return "Masculine"))

(fn `GetParticipantIcon`
  (params (ActiveSpeaker :type Name) (ActiveSpeakerState :type Name))
  (returns (ReturnValue :type "Texture2D Object Reference"))
  (return (`self.PlayerIcon`)))

(fn `GetParticipantName`
  (returns (ReturnValue :type Name))
  (return (`self.PlayerName`)))

(fn `ModifyBoolValue`
  (params (ValueName :type Name) (bNewValue :type Boolean))
  (returns (ReturnValue :type Boolean))
  (return false))

(fn `ModifyFloatValue`
  (params (ValueName :type Name) (bDelta :type Boolean) (Value :type "Float (double-precision)"))
  (returns (ReturnValue :type Boolean))
  (return false))

(fn `ModifyIntValue`
  (params (ValueName :type Name) (bDelta :type Boolean) (Value :type Integer))
  (returns (ReturnValue :type Boolean))
  (return false))

(fn `ModifyNameValue`
  (params (ValueName :type Name) (NameValue :type Name))
  (returns (ReturnValue :type Boolean))
  (return false))

(fn `OnDialogueEvent`
  (params (Context :type "DlgContext Object Reference") (EventName :type Name))
  (returns (ReturnValue :type Boolean))
  (return false))

(fn `SelectDialogueOption`
  (params (OptionIndex :type Integer))
  (bind _returnvalue (`GameplayStatics.GetPlayerController` 0))
  (`/Engine/EditorBlueprintResources/StandardMacros.IsValid` (`self.ActiveContext`)
    (:`Is Valid`
      (bind _returnvalue_2 (`DlgContext.ChooseOption` (`self.ActiveContext`) OptionIndex))
      (if _returnvalue_2
        ;[1 1 1] Dialogue still active - Refresh UI
        (`/Game/Widgets/UI_Dialogue.Refresh` (`self.DialogueWidget`) (`self.ActiveContext`))
        (else
          ;[1 1 1] Dialogue ended - hide UI + leave dialogue mode
          (`/Game/Widgets/UI_Dialogue.Refresh` (`self.DialogueWidget`) null)
          (`WidgetBlueprintLibrary.SetInputMode_GameOnly` _returnvalue)
          (`self.EnableInput` _returnvalue)
          (set `PlayerController.bShowMouseCursor` false _returnvalue)
          (set `self.bInDialogue` false))))))

(fn `StartDialogue`
  (params (DialogueObject :type "DlgDialogue Object Reference"))
  (bind _returnvalue (`GameplayStatics.GetPlayerController` 0))
  (if (not (`self.bInDialogue`))
    (bind _returnvalue_2 (`DlgManager.StartDialogueWithDefaultParticipants` DialogueObject))
    (`/Engine/EditorBlueprintResources/StandardMacros.IsValid` _returnvalue_2
      (:`Is Valid`
        (bind _output_get (set `self.ActiveContext` _returnvalue_2))
        (`/Game/Widgets/UI_Dialogue.Refresh` (`self.DialogueWidget`) _output_get)
        (`WidgetBlueprintLibrary.SetInputMode_GameAndUIEx` _returnvalue null)
        (`self.DisableInput` _returnvalue)
        (set `PlayerController.bShowMouseCursor` true _returnvalue)
        (set `self.bInDialogue` true)))))

(fn `UserConstructionScript`)